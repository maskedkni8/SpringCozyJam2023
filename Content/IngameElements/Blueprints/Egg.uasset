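; Egg actor: a colored physics object that responds to being lifted and dropped.
; On BeginPlay it writes MyColor into the Sphere's "Color" material parameter, feeding blue to X and red to Z, so the channels are in reversed order.
; On_Lift turns off physics simulation on the Sphere, and On_Drop turns it back on.
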(event `self.ReceiveBeginPlay`
  (bind (_mycolor_b _mycolor_g _mycolor_r) (break `Color` (`self.MyColor`)))
  (`MeshComponent.SetVectorParameterValueOnMaterials` (`self.Sphere`) "Color" (`KismetMathLibrary.MakeVector` (`KismetMathLibrary.Conv_ByteToDouble` _mycolor_b) (`KismetMathLibrary.Conv_ByteToDouble` _mycolor_g) (`KismetMathLibrary.Conv_ByteToDouble` _mycolor_r))))

(event `On_Lift`
  (`PrimitiveComponent.SetSimulatePhysics` (`self.Sphere`) false))

(event `On_Drop`
  (`PrimitiveComponent.SetSimulatePhysics` (`self.Sphere`) true))

(fn `UserConstructionScript`)