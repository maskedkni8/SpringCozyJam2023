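; Egg pedestal that lights up when an egg carrying its ConnectedTag rests in its box.
; Every Tick it scans Box for overlapping Egg actors and switches the Holder material between on and off looks.
; A matching egg also sets HoldingEgg, which this graph never clears.
; The begin and end overlap events are empty, with older material-switch logic left unconnected.
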(event `self.ReceiveActorBeginOverlap`
  (params (OtherActor :type "Actor Object Reference"))
  ;[1 1 1] Ech If egg on
)

(event `self.ReceiveTick`
  (params (DeltaSeconds :type "Float (single-precision)"))
  (bind _holder (`self.Holder`))
  (bind _overlappingactors (`PrimitiveComponent.GetOverlappingActors` (`self.Box`) "/Game/IngameElements/Blueprints/Egg.Egg_C"))
  (if (== (`KismetArrayLibrary.Array_Length` _overlappingactors) 0)
    (`PrimitiveComponent.SetMaterial` _holder 0 (`self.TurnedOFF_Mat`) :!label _label)
    (else
      (for _array_element _overlappingactors
        (if (`self.ActorHasTag` _array_element (`self.ConnectedTag`))
          (`PrimitiveComponent.SetMaterial` _holder 0 (`self.TurnedON_Mat`))
          (set `self.HoldingEgg` true)
          (break)
          (else
            (goto _label)))))))

(event `self.ReceiveActorEndOverlap`
  (params (OtherActor :type "Actor Object Reference"))
  ;[1 1 1] Check Egg OFF
)

(fn `UserConstructionScript`)