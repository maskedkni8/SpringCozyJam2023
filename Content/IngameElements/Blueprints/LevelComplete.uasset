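; Level goal actor that shows whether every EggPedestal in the level holds an egg.
; It gathers all pedestals at BeginPlay, and the CheckForGameOver event sets the completion flag from their HoldingEgg states.
; Tick switches the Cone's material between win and lose to match that flag.
; An overlapping Bunny plays its win regardless of the flag, as that branch's condition is hardcoded true.
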(event `CheckForGameOver`
  (set `self.LoopBool` true)
  (for _array_element (`self.EggPedestal`)
    (bind _output_get (set `self.LoopBool` (== (`/Game/IngameElements/Blueprints/EggPedestal.HoldingEgg` _array_element) (`self.LoopBool`))))
    (if (not _output_get)
      (break)))
  (set `self.Level COmplete` (`self.LoopBool`)))

(event `self.ReceiveBeginPlay`
  (bind _outactors (`GameplayStatics.GetAllActorsOfClass` "/Game/IngameElements/Blueprints/EggPedestal.EggPedestal_C"))
  (set `self.EggPedestal` _outactors))

(event `self.ReceiveActorBeginOverlap`
  (params (OtherActor :type "Actor Object Reference"))
  (bind _asbunny (cast `/Game/IngameElements/Blueprints/Bunny` OtherActor))
  (if true
    (`/Game/IngameElements/Blueprints/Bunny.Play Win` _asbunny)))

(event `self.ReceiveTick`
  (params (DeltaSeconds :type "Float (single-precision)"))
  (if (`self.Level COmplete`)
    (`PrimitiveComponent.SetMaterial` (`self.Cone`) 0 (`self.WinMaterial`))
    (else
      (`PrimitiveComponent.SetMaterial` (`self.Cone`) 0 (`self.LoseMaterial`)))))

(fn `CheckAndTrue`
  (params (Check :type Boolean))
  (returns (NewParam :type Boolean))
  (return (and Check true)))

(fn `UserConstructionScript`)