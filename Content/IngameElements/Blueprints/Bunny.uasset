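; Bunny player character that carries eggs, plays a win montage with input disabled, and reacts to hard landings.
; Interact picks up an overlapping "Egg"-tagged actor onto the mesh's HoldSocket or drops the held one, notifying the Egg each way.
; Movement mode changes and a delayed CheckSpeed re-check flag fast falls, then play a landing montage on Walking, disabling and immediately restoring movement.
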(event `EnhancedInput|/Game/IngameElements/Input/Actions/IA_Interact`
  (params (ActionValue :type Boolean) (ElapsedSeconds :type "Float (double-precision)") (TriggeredSeconds :type "Float (double-precision)") (InputAction :type "InputAction Object Reference" :default "/Game/IngameElements/Input/Actions/IA_Interact.IA_Interact"))
  ;[1 1 1] PickUp
  (:`Completed`
    (if (not (`self.IsHolding`))
      (for _array_element (`PrimitiveComponent.GetOverlappingActors` (`self.PickUpCheck`) "/Script/Engine.Actor")
        (if (`self.ActorHasTag` _array_element "Egg")
          (bind _output_get (set `self.HeldItem` _array_element))
          (bind _asegg (cast `/Game/IngameElements/Blueprints/Egg` _output_get))
          (`/Game/IngameElements/Blueprints/Egg.On_Lift` _asegg)
          (`self.K2_AttachToComponent` _output_get (`self.Mesh`) "HoldSocket" "SnapToTarget" "SnapToTarget" "KeepWorld" true)
          (`KismetSystemLibrary.Delay` 0.2)
          (set `self.IsHolding` true))))))

(event `Play Win`
  (`self.DisableInput` (`GameplayStatics.GetPlayerController` 0))
  (`|PlayMontage` null "/Game/Characters/Bunny/BunnyV2/WInMont.WInMont"))

(event `EnhancedInput|/Game/IngameElements/Input/Actions/IA_Interact`
  (params (ActionValue :type Boolean) (ElapsedSeconds :type "Float (double-precision)") (TriggeredSeconds :type "Float (double-precision)") (InputAction :type "InputAction Object Reference" :default "/Game/IngameElements/Input/Actions/IA_Interact.IA_Interact"))
  (bind _helditem (`self.HeldItem`))
  ;[1 1 1] Drop
  (:`Completed`
    (if (`self.IsHolding`)
      (`self.K2_DetachFromActor` _helditem "KeepWorld" "KeepWorld" "KeepWorld")
      (set `self.IsHolding` false)
      (bind _asegg (cast `/Game/IngameElements/Blueprints/Egg` _helditem))
      (`/Game/IngameElements/Blueprints/Egg.On_Drop` _asegg))))

(event `CheckSpeed`
  (bind (_returnvalue_x _returnvalue_y _returnvalue_z) (`KismetMathLibrary.BreakVector` (`self.GetVelocity`)))
  (bind _charactermovement (`self.CharacterMovement`))
  ;[1 1 1] Fall
  (`|ExecutionSequence` :!label _label
    (:`then_0`
      (if (`|EnumEquality` (stale `self.K2_OnMovementModeChanged` NewMovementMode) "MOVE_Falling")
        (set `self.HardLand` (<= _returnvalue_z -50.0))
        (else
          (`KismetSystemLibrary.Delay` 0.2)
          (`self.CheckSpeed`))))
    (:`then_1`
      (if (and (`|EnumEquality` (stale `self.K2_OnMovementModeChanged` NewMovementMode) "MOVE_Walking") (`self.HardLand`))
        (`CharacterMovementComponent.DisableMovement` _charactermovement)
        (`self.PlayAnimMontage` "/Game/Characters/Bunny/BunnyV2/Landing_Anim_Montage.Landing_Anim_Montage")
        (set `self.HardLand` false)
        (`CharacterMovementComponent.SetMovementMode` _charactermovement "MOVE_Walking" 0)))))

(event `self.K2_OnMovementModeChanged`
  (params (PrevMovementMode :type "EMovementMode Enum" :default "MOVE_None") (NewMovementMode :type "EMovementMode Enum" :default "MOVE_None") (PrevCustomMode :type Byte) (NewCustomMode :type Byte))
  ;[1 1 1] Fall
  (goto _label))

(fn `UserConstructionScript`)